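; Slime mob Blueprint that handles taking damage, dying and attacking.
; Incoming damage passes a DoOnce gate, lowers health and plays hurt feedback, ignoring further hits until the montage-length delay ends.
; Death plays a sound, detaches the controller and disables capsule collision, leaving the gate closed.
; Attack trigger starts a short, cancellable one-shot timer, then sphere-traces between mesh sockets and damages the hit actor.
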(event `self.ReceiveAnyDamage`
  (params (Damage :type "Float (single-precision)") (DamageType :type "DamageType Object Reference") (InstigatedBy :type "Controller Object Reference") (DamageCauser :type "Actor Object Reference"))
  ;[1 1 1] Handle slime taking damage
  (`/Engine/EditorBlueprintResources/StandardMacros.DoOnce` false :!label _label
    (:`Completed`
      (bind _output_get (set `HealthComponent.CurrentHealth` (- (`HealthComponent.CurrentHealth` (`self.Health`)) Damage) (`self.Health`)))
      (if (not (<= _output_get 0.0))
        (`GameplayStatics.PlaySound2D` "/Game/Blueprints/Mobs/Slime/SC_SlimeDamaged.SC_SlimeDamaged" 1.0 1.0 0.0 null null)
        (bind _returnvalue (`self.PlayAnimMontage` "/Game/Blueprints/Mobs/Slime/AM_SlimeDamaged.AM_SlimeDamaged"))
        (`KismetSystemLibrary.Delay` _returnvalue)
        (goto _label :!via `Reset`)
        (else
          (`GameplayStatics.PlaySound2D` "/Game/Blueprints/Mobs/Slime/SlimeDeath.SlimeDeath" 1.0 1.0 0.0 null null)
          (`self.DetachFromControllerPendingDestroy`)
          (`PrimitiveComponent.SetCollisionEnabled` (`self.CapsuleComponent`) "NoCollision"))))))

(event `TriggerSlimeAttack`
  ;[1 1 1] Handle slime attack
  (bind _returnvalue (`KismetSystemLibrary.K2_SetTimerDelegate` (delegate `SlimeAttackTrace`) 0.1))
  (set `self.SlimeAttackTimer` _returnvalue))

(event `SlimeAttackTrace`
  ;[1 1 1] Handle slime attack
  (bind _outhit (`KismetSystemLibrary.SphereTraceSingle` :`Start` (`SceneComponent.GetSocketLocation` (`self.Mesh`) "AttackStart") :`End` (`SceneComponent.GetSocketLocation` (`self.Mesh`) "AttackEnd") :`Radius` 300.0 :`TraceChannel` "TraceTypeQuery4" :`TraceColor` (struct :`A` 1.0)))
  (`GameplayStatics.ApplyDamage` (`.HitActor` (`GameplayStatics.BreakHitResult` _outhit)) 10.0))

(event `StopSlimeAttack`
  ;[1 1 1] Handle slime attack
  (`KismetSystemLibrary.K2_InvalidateTimerHandle` (`self.SlimeAttackTimer`)))

(fn `UserConstructionScript`)