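; Animation notify state that marks the window of the Dualblade hero's first attack during which the blade line trace runs.
; Begin and end cast the mesh owner to BP_Dualblade, then call TriggerAttack1 and StopAttack1 on BP_DualBladeController.
; Begin fetches that controller as player controller 0, while end takes the hero's own controller.
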(fn `Received_NotifyBegin`
  (params (MeshComp :type "SkeletalMeshComponent Object Reference") (Animation :type "AnimSequenceBase Object Reference") (TotalDuration :type "Float (single-precision)") (EventReference :type "AnimNotifyEventReference Structure (by ref)"))
  (returns (ReturnValue :type Boolean))
  ;[1 1 1] Trigger the attack 1 blade linetrace
  (bind _asbp_dualblade (cast `/Game/Blueprints/Heros/Dualblade/BP_Dualblade` (`ActorComponent.GetOwner` MeshComp)))
  (bind _asbp_dual_blade_controller (cast `/Game/Blueprints/Controllers/PlayerControllers/BP_DualBladeController` (`GameplayStatics.GetPlayerController` _asbp_dualblade)))
  (`/Game/Blueprints/Controllers/PlayerControllers/BP_DualBladeController.TriggerAttack1` _asbp_dual_blade_controller)
  (return false))

(fn `Received_NotifyEnd`
  (params (MeshComp :type "SkeletalMeshComponent Object Reference") (Animation :type "AnimSequenceBase Object Reference") (EventReference :type "AnimNotifyEventReference Structure (by ref)"))
  (returns (ReturnValue :type Boolean))
  ;[1 1 1] Stop the attack 1 blade linetrace
  (bind _asbp_dualblade (cast `/Game/Blueprints/Heros/Dualblade/BP_Dualblade` (`ActorComponent.GetOwner` MeshComp)))
  (bind _asbp_dual_blade_controller (cast `/Game/Blueprints/Controllers/PlayerControllers/BP_DualBladeController` (`Pawn.GetController` _asbp_dualblade)))
  (`/Game/Blueprints/Controllers/PlayerControllers/BP_DualBladeController.StopAttack1` _asbp_dual_blade_controller)
  (return false))