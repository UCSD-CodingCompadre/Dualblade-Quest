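; Player controller for the Dualblade character, handling three sword attacks and returning to the main menu on Escape.
; Each attack input plays a sound and montage, with shared playing flags preventing overlap; Attack 3 is restricted to Quest 2 and 3 game modes.
; Externally callable Trigger events start looping timers that sphere-trace along a blade's sockets and apply damage, with a much wider radius for Attack 3.
; Matching Stop events clear those timers and flags.
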(event `self.ReceiveBeginPlay`
  ;[1 1 1] Set the character
  (bind _asbp_dualblade (cast `/Game/Blueprints/Heros/Dualblade/BP_Dualblade` (`GameplayStatics.GetPlayerPawn` 0)))
  (set `self.DualbladeCharacter` _asbp_dualblade))

(event `Key|Escape`
  (params (Key :type "Key Structure"))
  ;[1 1 1] Return to Main Menu
  (:`Pressed`
    (`GameplayStatics.OpenLevelBySoftObjectPtr` "/Game/Levels/MainMenu.MainMenu")))

(event `EnhancedInput|/Game/Blueprints/Input/IA_Attack3`
  (params (ActionValue :type Boolean) (ElapsedSeconds :type "Float (double-precision)") (TriggeredSeconds :type "Float (double-precision)") (InputAction :type "InputAction Object Reference" :default "/Game/Blueprints/Input/IA_Attack3.IA_Attack3"))
  (bind _returnvalue (`GameplayStatics.GetObjectClass` (`GameplayStatics.GetGameMode`)))
  ;[1 1 1] Handle the attack 3
  (:`Triggered`
    (if (and (not (`self.Attack1Playing`)) (not (`self.Attack2Playing`)) (not (`self.Attack3Playing`)) (or (== _returnvalue "/Game/Blueprints/GameModes/BP_Quest2GameMode.BP_Quest2GameMode_C") (== _returnvalue "/Game/Blueprints/GameModes/BP_Quest3GameMode.BP_Quest3GameMode_C")))
      (`/Engine/EditorBlueprintResources/StandardMacros.DoOnce` false :!label _label
        (:`Completed`
          (set `self.Attack3Playing` true)
          (`GameplayStatics.PlaySound2D` "/Game/Blueprints/Heros/Dualblade/SC_Attack3Sound.SC_Attack3Sound" 1.0 1.0 0.0 null null)
          (bind _returnvalue_2 (`Character.PlayAnimMontage` (`self.DualbladeCharacter`) "/Game/Blueprints/Heros/Dualblade/AM_DualBladeAttack3.AM_DualBladeAttack3" 1.0 "None"))
          (`KismetSystemLibrary.Delay` _returnvalue_2)
          (goto _label :!via `Reset`))))))

(event `EnhancedInput|/Game/Blueprints/Input/IA_Attack2`
  (params (ActionValue :type Boolean) (ElapsedSeconds :type "Float (double-precision)") (TriggeredSeconds :type "Float (double-precision)") (InputAction :type "InputAction Object Reference" :default "/Game/Blueprints/Input/IA_Attack2.IA_Attack2"))
  ;[1 1 1] Handle the attack 2
  (:`Triggered`
    (if (and (not (`self.Attack1Playing`)) (not (`self.Attack2Playing`)) (not (`self.Attack3Playing`)))
      (`/Engine/EditorBlueprintResources/StandardMacros.DoOnce` false :!label _label_2
        (:`Completed`
          (set `self.Attack2Playing` true)
          (`GameplayStatics.PlaySound2D` "/Game/Blueprints/Heros/Dualblade/SC_Attack2Sound.SC_Attack2Sound" 1.0 1.0 0.0 null null)
          (bind _returnvalue (`Character.PlayAnimMontage` (`self.DualbladeCharacter`) "/Game/Blueprints/Heros/Dualblade/AM_DualBladeAttack2.AM_DualBladeAttack2" 1.0 "None"))
          (`KismetSystemLibrary.Delay` _returnvalue)
          (goto _label_2 :!via `Reset`))))))

(event `EnhancedInput|/Game/Blueprints/Input/IA_Attack1`
  (params (ActionValue :type Boolean) (ElapsedSeconds :type "Float (double-precision)") (TriggeredSeconds :type "Float (double-precision)") (InputAction :type "InputAction Object Reference" :default "/Game/Blueprints/Input/IA_Attack1.IA_Attack1"))
  ;[1 1 1] Handle the attack 1 input
  (:`Triggered`
    (if (and (not (`self.Attack1Playing`)) (not (`self.Attack2Playing`)) (not (`self.Attack3Playing`)))
      (`/Engine/EditorBlueprintResources/StandardMacros.DoOnce` false :!label _label_3
        (:`Completed`
          (set `self.Attack1Playing` true)
          (`GameplayStatics.PlaySound2D` "/Game/Blueprints/Heros/Dualblade/SC_Attack1Sound.SC_Attack1Sound" 1.0 1.0 0.0 null null)
          (bind _returnvalue (`Character.PlayAnimMontage` (`self.DualbladeCharacter`) "/Game/Blueprints/Heros/Dualblade/AM_DualbladeAttack1.AM_DualbladeAttack1" 1.0 "None"))
          (`KismetSystemLibrary.Delay` _returnvalue)
          (goto _label_3 :!via `Reset`))))))

(event `TriggerAttack1`
  ;[1 1 1] Handle the attack 1 line trace
  (bind _returnvalue (`KismetSystemLibrary.K2_SetTimerDelegate` (delegate `Attack1BladeLineTrace`) 0.01 true))
  (set `self.Attack1TriggerEvent` _returnvalue))

(event `TriggerAttack2`
  ;[1 1 1] Handle the attack 2 line trace
  (bind _returnvalue (`KismetSystemLibrary.K2_SetTimerDelegate` (delegate `Attack2LineTrace`) 0.1 true))
  (set `self.Attack2TriggerEvent` _returnvalue))

(event `Attack1BladeLineTrace`
  (bind _leftblade (`DualBlade.LeftBlade` (`self.DualbladeCharacter`)))
  ;[1 1 1] Handle the attack 1 line trace
  (bind _outhit (`KismetSystemLibrary.SphereTraceSingle` :`Start` (`SceneComponent.GetSocketLocation` _leftblade "SwordTip") :`End` (`SceneComponent.GetSocketLocation` _leftblade "SwordEnd") :`Radius` 25.0 :`TraceChannel` "TraceTypeQuery3" :`bIgnoreSelf` false :`TraceColor` (struct :`A` 1.0)))
  (`GameplayStatics.ApplyDamage` (`.HitActor` (`GameplayStatics.BreakHitResult` _outhit)) 25.0))

(event `Attack2LineTrace`
  (bind _rightblade (`DualBlade.RightBlade` (`self.DualbladeCharacter`)))
  ;[1 1 1] Handle the attack 2 line trace
  (bind _outhit (`KismetSystemLibrary.SphereTraceSingle` :`Start` (`SceneComponent.GetSocketLocation` _rightblade "SwordTip") :`End` (`SceneComponent.GetSocketLocation` _rightblade "SwordEnd") :`Radius` 40.0 :`TraceChannel` "TraceTypeQuery3" :`TraceColor` (struct :`A` 1.0) :`TraceHitColor` (struct :`R` 0.822917 :`G` 0.13958 :`B` 0.074002 :`A` 1.0)))
  (if true
    (`GameplayStatics.ApplyDamage` (`.HitActor` (`GameplayStatics.BreakHitResult` _outhit)) 25.0)))

(event `TriggerAttack3`
  ;[1 1 1] Handle the attack 3 line trace
  (bind _returnvalue (`KismetSystemLibrary.K2_SetTimerDelegate` (delegate `Attack3LineTrace`) 0.1 true))
  (set `self.Attack3TriggerEvent` _returnvalue))

(event `Attack3LineTrace`
  (bind _leftblade (`DualBlade.LeftBlade` (`self.DualbladeCharacter`)))
  ;[1 1 1] Handle the attack 3 line trace
  (bind _outhit (`KismetSystemLibrary.SphereTraceSingle` :`Start` (`SceneComponent.GetSocketLocation` _leftblade "SwordTip") :`End` (`SceneComponent.GetSocketLocation` _leftblade "SwordEnd") :`Radius` 200.0 :`TraceChannel` "TraceTypeQuery3" :`TraceColor` (struct :`A` 1.0) :`TraceHitColor` (struct :`R` 0.822917 :`G` 0.13958 :`B` 0.074002 :`A` 1.0)))
  (if true
    (`GameplayStatics.ApplyDamage` (`.HitActor` (`GameplayStatics.BreakHitResult` _outhit)) 25.0)))

(event `StopAttack2`
  ;[1 1 1] Handle the attack 2 line trace
  (set `self.Attack2Playing` false)
  (`KismetSystemLibrary.K2_ClearAndInvalidateTimerHandle` (`self.Attack2TriggerEvent`)))

(event `StopAttack1`
  ;[1 1 1] Handle the attack 1 line trace
  (set `self.Attack1Playing` false)
  (`KismetSystemLibrary.K2_ClearAndInvalidateTimerHandle` (`self.Attack1TriggerEvent`)))

(event `StopAttack3`
  ;[1 1 1] Handle the attack 3 line trace
  (set `self.Attack3Playing` false)
  (`KismetSystemLibrary.K2_ClearAndInvalidateTimerHandle` (`self.Attack3TriggerEvent`)))

(fn `UserConstructionScript`)