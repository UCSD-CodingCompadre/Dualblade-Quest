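; BP_Stump is the Blueprint for the Stump mob, handling damage, death and a melee attack.
; A DoOnce gate ignores further hits while the damaged montage plays; at zero health it plays a death sound, detaches the controller and disables capsule collision.
; TriggerStumpAttack starts a short one-shot timer for a sphere trace between mesh sockets that applies damage to the hit actor; StopStumpAttack cancels that timer.
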(event `self.ReceiveAnyDamage`
  (params (Damage :type "Float (single-precision)") (DamageType :type "DamageType Object Reference") (InstigatedBy :type "Controller Object Reference") (DamageCauser :type "Actor Object Reference"))
  ;[1 1 1] Handle taking damage
  (`/Engine/EditorBlueprintResources/StandardMacros.DoOnce` false :!label _label
    (:`Completed`
      (bind _output_get (set `HealthComponent.CurrentHealth` (- (`HealthComponent.CurrentHealth` (`self.Health`)) Damage) (`self.Health`)))
      (if (<= _output_get 0.0)
        (`GameplayStatics.PlaySound2D` "/Game/Blueprints/Mobs/Stump/SC_StumpDeath.SC_StumpDeath" 1.0 1.0 0.0 null null)
        (`self.DetachFromControllerPendingDestroy`)
        (`PrimitiveComponent.SetCollisionEnabled` (`self.CapsuleComponent`) "NoCollision")
        (else
          (`GameplayStatics.PlaySound2D` "/Game/Blueprints/Mobs/Stump/SC_StumpDamaged.SC_StumpDamaged" 1.0 1.0 0.0 null null)
          (bind _returnvalue (`self.PlayAnimMontage` "/Game/Blueprints/Mobs/Stump/AM_StumpDamaged.AM_StumpDamaged"))
          (`KismetSystemLibrary.Delay` _returnvalue)
          (goto _label :!via `Reset`))))))

(event `TriggerStumpAttack`
  ;[1 1 1] Handle stump attack
  (bind _returnvalue (`KismetSystemLibrary.K2_SetTimerDelegate` (delegate `StumpAttackTrace`) 0.1))
  (set `self.StumpAttackTimer` _returnvalue))

(event `StumpAttackTrace`
  ;[1 1 1] Handle stump attack
  (bind _outhit (`KismetSystemLibrary.SphereTraceSingle` :`Start` (`SceneComponent.GetSocketLocation` (`self.Mesh`) "AttackStart") :`End` (`SceneComponent.GetSocketLocation` (`self.Mesh`) "AttackEnd") :`Radius` 300.0 :`TraceChannel` "TraceTypeQuery4" :`TraceColor` (struct :`A` 1.0)))
  (`GameplayStatics.ApplyDamage` (`.HitActor` (`GameplayStatics.BreakHitResult` _outhit)) 20.0))

(event `StopStumpAttack`
  ;[1 1 1] Handle stump attack
  (`KismetSystemLibrary.K2_InvalidateTimerHandle` (`self.StumpAttackTimer`)))

(fn `UserConstructionScript`)