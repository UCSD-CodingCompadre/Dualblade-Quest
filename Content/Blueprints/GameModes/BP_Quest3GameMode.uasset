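; Game mode for Quest 3 that runs a clear-the-campsite objective, a Stump boss fight and the credits transition.
; BeginPlay starts music, shows HUD widgets and gathers all BP_Stump actors for the quest count.
; Tick polls health to restart the level on hero death, remove dead mobs and update the quest log.
; Once stumps are cleared, it resets hero health, swaps music, spawns the AI boss and tracks its health bar until victory.
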(event `self.ReceiveBeginPlay`
  ;[1 1 1] Set the mob count
  (bind _returnvalue (`GameplayStatics.CreateSound2D` "/Game/Blueprints/Music/SC_Quest3Music.SC_Quest3Music" 1.0 1.0 0.0 null))
  (bind _output_get (set `self.QuestMusic` _returnvalue))
  (`AudioComponent.Play` _output_get 0.0)
  (`self.DisplayHealthBar`)
  (bind _outactors (`GameplayStatics.GetAllActorsOfClass` "/Game/Blueprints/Mobs/Stump/BP_Stump.BP_Stump_C"))
  (bind _output_get_2 (set `self.Mobs` _outactors))
  (bind _output_get_3 (set `self.TotalMobs` (`KismetArrayLibrary.Array_Length` _output_get_2)))
  (set `self.ActiveMobs` _output_get_3)
  (bind _returnvalue_2 (`|CreateWidget` "/Game/Blueprints/Widgets/WBP_TutorialMessage3.WBP_TutorialMessage3_C"))
  (`UserWidget.AddToViewport` _returnvalue_2 0)
  (`KismetSystemLibrary.Delay` 5.0)
  (`Widget.RemoveFromParent` _returnvalue_2)
  (bind _returnvalue_3 (`|CreateWidget` "/Game/Blueprints/Widgets/WBP_ActiveQuest.WBP_ActiveQuest_C" (`GameplayStatics.GetPlayerController` 0)))
  (set `self.QuestLog` _returnvalue_3)
  (set `TextBlock.Text` "Clear the campsite" (`/Game/Blueprints/Widgets/WBP_ActiveQuest.T_QuestName` (`self.QuestLog`)))
  (bind _questtask (`self.GetTaskString`))
  (set `TextBlock.Text` (`KismetTextLibrary.Conv_StringToText` _questtask) (`/Game/Blueprints/Widgets/WBP_ActiveQuest.T_QuestTask` (`self.QuestLog`)))
  (`UserWidget.AddToViewport` (`self.QuestLog`) 0))

(event `self.ReceiveTick`
  (params (DeltaSeconds :type "Float (single-precision)"))
  ;[1 1 1] Remove the dead mob and decrement active mobs
  (bind _isalive (`self.CheckHeroIsAlive`))
  (if (not _isalive)
    (bind _returnvalue (`|CreateWidget` "/Game/Blueprints/Widgets/WBP_QuestComplete.WBP_QuestComplete_C"))
    (set `TextBlock.Text` "Hero Dead. \nRestarting level..." (`/Game/Blueprints/Widgets/WBP_QuestComplete.T_Message` _returnvalue))
    (`UserWidget.AddToViewport` _returnvalue 0)
    (`GameplayStatics.OpenLevelBySoftObjectPtr` "/Game/Levels/Quest3.Quest3")
    (else
      (for _array_element (`self.Mobs`)
        (if (<= (`HealthComponent.CurrentHealth` (`/Game/Blueprints/Mobs/Stump/BP_Stump.Health` _array_element)) 0.0)
          (bind _returnvalue_2 (`KismetArrayLibrary.Array_RemoveItem` (`self.Mobs`) _array_element))
          (if _returnvalue_2
            (set `self.ActiveMobs` (- (`self.ActiveMobs`) 1))
            (bind _questtask (`self.GetTaskString`))
            (set `TextBlock.Text` (`KismetTextLibrary.Conv_StringToText` _questtask) (`/Game/Blueprints/Widgets/WBP_ActiveQuest.T_QuestTask` (`self.QuestLog`))))))
      (if (and (== (`self.ActiveMobs`) 0) (not (`self.InBossBattle`)))
        (`/Engine/EditorBlueprintResources/StandardMacros.DoOnce` false
          (:`Completed`
            (`Widget.RemoveFromParent` (`self.QuestLog`))
            (bind _returnvalue_3 (`|CreateWidget` "/Game/Blueprints/Widgets/WBP_TutorialMessage3.WBP_TutorialMessage3_C" (`GameplayStatics.GetPlayerController` 0)))
            (set `TextBlock.Text` "Uh oh. I think there is something  \nbigger coming to stop us. \nYou got this!" (`/Game/Blueprints/Widgets/WBP_TutorialMessage3.T_Message` _returnvalue_3))
            (`UserWidget.AddToViewport` _returnvalue_3 0)
            (bind _asbp_dualblade (cast `/Game/Blueprints/Heros/Dualblade/BP_Dualblade` (`GameplayStatics.GetPlayerPawn` 0)))
            (set `HealthComponent.CurrentHealth` 1000.0 (`/Game/Blueprints/Heros/Dualblade/BP_Dualblade.Health` _asbp_dualblade))
            (`KismetSystemLibrary.Delay` 5.0)
            (`Widget.RemoveFromParent` _returnvalue_3)
            (`AudioComponent.Stop` (`self.QuestMusic`))
            (`GameplayStatics.PlaySound2D` "/Game/Blueprints/Music/SC_Quest3BossMusic.SC_Quest3BossMusic" 1.0 1.0 0.0 null null)
            (set `self.InBossBattle` true)
            (set `self.IsBossAlive` true)
            (bind _returnvalue_4 (`AIBlueprintHelperLibrary.SpawnAIFromClass` "/Game/Blueprints/Mobs/Stump/BP_StumpBoss.BP_StumpBoss_C" "/Game/Blueprints/AI/BT_MobAI.BT_MobAI" (`self.Location`) (struct) false null))
            (bind _asbp_stump_boss (cast `/Game/Blueprints/Mobs/Stump/BP_StumpBoss` _returnvalue_4))
            (`|ExecutionSequence`
              (:`then_0`
                (bind _output_get (set `self.BP_StumpBoss` _asbp_stump_boss))
                (bind _asbp_mob_aicontroller (cast `/Game/Blueprints/AI/BP_MobAIController` (`Pawn.GetController` _output_get)))
                (`BlackboardComponent.SetValueAsVector` (`AIBlueprintHelperLibrary.GetBlackboard` _asbp_mob_aicontroller) "AIPawnStartLocation" (`self.Location`))
                (set `HealthComponent.CurrentHealth` 750.0 (`/Game/Blueprints/Mobs/Stump/BP_Stump.Health` _output_get)))
              (:`then_1`
                (bind _returnvalue_5 (`|CreateWidget` "/Game/Blueprints/Widgets/WBP_BossHealthbar.WBP_BossHealthbar_C"))
                (bind _output_get_2 (set `self.WBP_BossHealthBar` _returnvalue_5))
                (`ProgressBar.SetPercent` (`/Game/Blueprints/Widgets/WBP_BossHealthbar.PB_HealthBar` _output_get_2) (/ (`HealthComponent.CurrentHealth` (`/Game/Blueprints/Mobs/Stump/BP_Stump.Health` (`self.BP_StumpBoss`))) 750.0))
                (`UserWidget.AddToViewport` (`self.WBP_BossHealthBar`) 0))
              (:`then_2`
                (set `TextBlock.Text` "Defeat Stump Boss" (`/Game/Blueprints/Widgets/WBP_ActiveQuest.T_QuestName` (`self.QuestLog`)))
                (set `TextBlock.Text` "1 /1 Stump \nBosse(s) Defeated" (`/Game/Blueprints/Widgets/WBP_ActiveQuest.T_QuestTask` (`self.QuestLog`)))
                (`UserWidget.AddToViewport` (`self.QuestLog`) 0)))))
        (elif (and (`self.IsBossAlive`) (`self.InBossBattle`))
          (bind _bp_stumpboss (`self.BP_StumpBoss`)
            (:`then`
              (if (not (<= (`HealthComponent.CurrentHealth` (`/Game/Blueprints/Mobs/Stump/BP_Stump.Health` _bp_stumpboss)) 0.0))
                (`ProgressBar.SetPercent` (`/Game/Blueprints/Widgets/WBP_BossHealthbar.PB_HealthBar` (`self.WBP_BossHealthBar`)) (/ (`HealthComponent.CurrentHealth` (`/Game/Blueprints/Mobs/Stump/BP_Stump.Health` (`self.BP_StumpBoss`))) 500.0))
                (else
                  (`ProgressBar.SetPercent` (`/Game/Blueprints/Widgets/WBP_BossHealthbar.PB_HealthBar` (`self.WBP_BossHealthBar`)) 0.0)
                  (`/Engine/EditorBlueprintResources/StandardMacros.DoOnce` false
                    (:`Completed`
                      (`Widget.RemoveFromParent` (`self.QuestLog`))
                      (bind _returnvalue_6 (`|CreateWidget` "/Game/Blueprints/Widgets/WBP_TutorialMessage3.WBP_TutorialMessage3_C"))
                      (bind _t_message (`/Game/Blueprints/Widgets/WBP_TutorialMessage3.T_Message` _returnvalue_6))
                      (set `TextBlock.Text` "You win!  \nThanks for playing" _t_message)
                      (`UserWidget.AddToViewport` _returnvalue_6 0)
                      (`KismetSystemLibrary.Delay` 5.0)
                      (set `TextBlock.Text` "Loading Credits..." _t_message)
                      (`KismetSystemLibrary.Delay` 5.0)
                      (`GameplayStatics.OpenLevelBySoftObjectPtr` "/Game/Levels/Credits.Credits"))))))
            (:`else`)))))))

(fn `CheckHeroIsAlive`
  (returns (IsAlive :type Boolean))
  ;[1 1 1] Check hero health to see if they are alive
  (bind _asbp_dualblade (cast `/Game/Blueprints/Heros/Dualblade/BP_Dualblade` (`GameplayStatics.GetPlayerPawn` 0))
    (:`then`
      (return (not (<= (`HealthComponent.CurrentHealth` (`/Game/Blueprints/Heros/Dualblade/BP_Dualblade.Health` _asbp_dualblade)) 0.0))))
    (:`CastFailed`
      (return false))))

(fn `DisplayHealthBar`
  ;[1 1 1] Display the health bar
  (bind _returnvalue (`|CreateWidget` "/Game/Blueprints/Widgets/WBP_Healthbar.WBP_Healthbar_C" (`GameplayStatics.GetPlayerController` 0)))
  (`UserWidget.AddToViewport` _returnvalue 0)
  (return))

(fn `GetTaskString`
  (returns (QuestTask :type String))
  ;[1 1 1] Create Task String
  (return (`KismetStringLibrary.Concat_StrStr` (`KismetStringLibrary.Conv_IntToString` (`self.ActiveMobs`)) " / " (`KismetStringLibrary.Conv_IntToString` (`self.TotalMobs`)) " Stumps left")))

(fn `UserConstructionScript`)