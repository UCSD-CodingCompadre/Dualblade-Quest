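; Game mode for Quest 1, "Defend the Farm", where the hero must kill every mushroom mob in the level.
; BeginPlay shows the health bar, counts the BP_Mushroom actors and shows a timed tutorial message before creating the quest log.
; Tick polls health to prune dead mobs and update the log, restarting the level if the hero dies.
; When no mobs remain, a DoOnce shows the completion widget, then loads Quest 2.
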(event `self.ReceiveBeginPlay`
  ;[1 1 1] Set the mob count
  (`self.DisplayHealthBar`)
  (bind _outactors (`GameplayStatics.GetAllActorsOfClass` "/Game/Blueprints/Mobs/Mushroom/BP_Mushroom.BP_Mushroom_C"))
  (bind _output_get (set `self.MushroomMobs` _outactors))
  (bind _output_get_2 (set `self.TotalMobs` (`KismetArrayLibrary.Array_Length` _output_get)))
  (set `self.ActiveMobs` _output_get_2)
  (bind _returnvalue (`|CreateWidget` "/Game/Blueprints/Widgets/WBP_TutorialMessage1.WBP_TutorialMessage1_C"))
  (`UserWidget.AddToViewport` _returnvalue 0)
  (`KismetSystemLibrary.Delay` 20.0)
  (`Widget.RemoveFromParent` _returnvalue)
  (bind _returnvalue_2 (`|CreateWidget` "/Game/Blueprints/Widgets/WBP_ActiveQuest.WBP_ActiveQuest_C" (`GameplayStatics.GetPlayerController` 0)))
  (set `self.QuestLog` _returnvalue_2)
  (set `TextBlock.Text` "Defend the Farm" (`/Game/Blueprints/Widgets/WBP_ActiveQuest.T_QuestName` (`self.QuestLog`)))
  (bind _questtask (`self.GetTaskString`))
  (set `TextBlock.Text` (`KismetTextLibrary.Conv_StringToText` _questtask) (`/Game/Blueprints/Widgets/WBP_ActiveQuest.T_QuestTask` (`self.QuestLog`)))
  (`UserWidget.AddToViewport` (`self.QuestLog`) 0))

(event `self.ReceiveTick`
  (params (DeltaSeconds :type "Float (single-precision)"))
  ;[1 1 1] Remove the dead mob and decrement active mobs
  (bind _isalive (`self.CheckHeroIsAlive`))
  (if (not _isalive)
    (bind _returnvalue (`|CreateWidget` "/Game/Blueprints/Widgets/WBP_QuestComplete.WBP_QuestComplete_C"))
    (set `TextBlock.Text` "Hero Dead. \nRestarting level..." (`/Game/Blueprints/Widgets/WBP_QuestComplete.T_Message` _returnvalue))
    (`UserWidget.AddToViewport` _returnvalue 0)
    (`GameplayStatics.OpenLevelBySoftObjectPtr` "/Game/Levels/Quest1.Quest1")
    (else
      (for _array_element (`self.MushroomMobs`)
        (if (<= (`HealthComponent.CurrentHealth` (`/Game/Blueprints/Mobs/Mushroom/BP_Mushroom.Health` _array_element)) 0.0)
          (bind _returnvalue_2 (`KismetArrayLibrary.Array_RemoveItem` (`self.MushroomMobs`) _array_element))
          (if _returnvalue_2
            (set `self.ActiveMobs` (- (`self.ActiveMobs`) 1))
            (bind _questtask (`self.GetTaskString`))
            (set `TextBlock.Text` (`KismetTextLibrary.Conv_StringToText` _questtask) (`/Game/Blueprints/Widgets/WBP_ActiveQuest.T_QuestTask` (`self.QuestLog`))))))
      (if (== (`self.ActiveMobs`) 0)
        (`/Engine/EditorBlueprintResources/StandardMacros.DoOnce` false :!label _label
          (:`Completed`
            (`Widget.RemoveFromParent` (`self.QuestLog`))
            (bind _returnvalue_3 (`|CreateWidget` "/Game/Blueprints/Widgets/WBP_QuestComplete.WBP_QuestComplete_C"))
            (bind _output_get (set `self.WBP_QuestComplete` _returnvalue_3))
            (`UserWidget.AddToViewport` _output_get 0)
            (`KismetSystemLibrary.Delay` 3.0)
            (set `TextBlock.Text` "Loading Quest 2" (`/Game/Blueprints/Widgets/WBP_QuestComplete.T_Message` (`self.WBP_QuestComplete`)))
            (`KismetSystemLibrary.Delay` 3.0)
            (`GameplayStatics.OpenLevelBySoftObjectPtr` "/Game/Levels/Quest2.Quest2")
            (goto _label :!via `Reset`)))))))

(fn `CheckHeroIsAlive`
  (returns (IsAlive :type Boolean))
  ;[1 1 1] Check hero health to see if they are alive
  (bind _asbp_dualblade (cast `/Game/Blueprints/Heros/Dualblade/BP_Dualblade` (`GameplayStatics.GetPlayerPawn` 0))
    (:`then`
      (return (not (<= (`HealthComponent.CurrentHealth` (`/Game/Blueprints/Heros/Dualblade/BP_Dualblade.Health` _asbp_dualblade)) 0.0))))
    (:`CastFailed`
      (return false))))

(fn `DisplayHealthBar`
  ;[1 1 1] Display the health bar
  (bind _returnvalue (`|CreateWidget` "/Game/Blueprints/Widgets/WBP_Healthbar.WBP_Healthbar_C" (`GameplayStatics.GetPlayerController` 0)))
  (`UserWidget.AddToViewport` _returnvalue 0)
  (return))

(fn `GetTaskString`
  (returns (QuestTask :type String))
  ;[1 1 1] Create Task String
  (return (`KismetStringLibrary.Concat_StrStr` (`KismetStringLibrary.Conv_IntToString` (`self.ActiveMobs`)) " / " (`KismetStringLibrary.Conv_IntToString` (`self.TotalMobs`)) " Mushrooms left")))

(fn `UserConstructionScript`)