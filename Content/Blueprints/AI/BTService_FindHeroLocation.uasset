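; Behavior tree service that tracks the hero's location while the player is within a mob's detection radius.
; Each tick it measures the distance from the AIPawnLocation blackboard value to the first player pawn.
; Within the fixed radius it writes the player's position to the HeroLocation key, and otherwise it clears that key.
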(event `self.ReceiveTick`
  (params (OwnerActor :type "Actor Object Reference") (DeltaSeconds :type "Float (single-precision)"))
  ;[1 1 1] Check if the hero is is in the detection radius of the mob
  (if (<= (`KismetMathLibrary.Vector_Distance` (`BTFunctionLibrary.GetBlackboardValueAsVector` (`self.AIPawnLocation`)) (`Actor.K2_GetActorLocation` (`GameplayStatics.GetPlayerPawn` 0))) 1500.0)
    (`BTFunctionLibrary.SetBlackboardValueAsVector` (`self.HeroLocation`) (`Actor.K2_GetActorLocation` (`GameplayStatics.GetPlayerPawn` 0)))
    (else
      (`BTFunctionLibrary.ClearBlackboardValue` (`self.HeroLocation`)))))