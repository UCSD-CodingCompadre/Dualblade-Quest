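; Mushroom mob Blueprint that handles taking damage, death and a sphere-trace attack.
; Damage reduces its Health value through a DoOnce, which resets after the hit-reaction montage delay, so hits during it are ignored.
; At zero health it plays a death sound, detaches its controller and disables capsule collision.
; Attack events start or cancel a short one-shot timer that sphere-traces between mesh sockets and damages the hit actor.
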(event `self.ReceiveAnyDamage`
  (params (Damage :type "Float (single-precision)") (DamageType :type "DamageType Object Reference") (InstigatedBy :type "Controller Object Reference") (DamageCauser :type "Actor Object Reference"))
  (bind _health (`self.Health`))
  ;[1 1 1] Handle taking damage
  (`/Engine/EditorBlueprintResources/StandardMacros.DoOnce` false :!label _label
    (:`Completed`
      (bind _output_get (set `HealthComponent.CurrentHealth` (- (`HealthComponent.CurrentHealth` _health) Damage) _health))
      (if (<= _output_get 0.0)
        (`GameplayStatics.PlaySound2D` "/Game/Blueprints/Mobs/Mushroom/SC_MushroomDeath.SC_MushroomDeath" 1.0 1.0 0.0 null null)
        (`self.DetachFromControllerPendingDestroy`)
        (`PrimitiveComponent.SetCollisionEnabled` (`self.CapsuleComponent`) "NoCollision")
        (else
          (`GameplayStatics.PlaySound2D` "/Game/Blueprints/Mobs/Mushroom/SC_MushroomDamaged.SC_MushroomDamaged" 1.0 1.0 0.0 null null)
          (bind _returnvalue (`self.PlayAnimMontage` "/Game/Blueprints/Mobs/Mushroom/AM_MushroomDamaged.AM_MushroomDamaged"))
          (`KismetSystemLibrary.Delay` _returnvalue)
          (goto _label :!via `Reset`))))))

(event `TriggerMushroomAttack`
  ;[1 1 1] Handle mushroom attack
  (bind _returnvalue (`KismetSystemLibrary.K2_SetTimerDelegate` (delegate `MushroomAttackTrace`) 0.1))
  (set `self.MushroomAttackTimer` _returnvalue))

(event `MushroomAttackTrace`
  ;[1 1 1] Handle mushroom attack
  (bind _outhit (`KismetSystemLibrary.SphereTraceSingle` :`Start` (`SceneComponent.GetSocketLocation` (`self.Mesh`) "AttackStart") :`End` (`SceneComponent.GetSocketLocation` (`self.Mesh`) "AttackEnd") :`Radius` 300.0 :`TraceChannel` "TraceTypeQuery4" :`TraceColor` (struct :`A` 1.0)))
  (`GameplayStatics.ApplyDamage` (`.HitActor` (`GameplayStatics.BreakHitResult` _outhit)) 5.0))

(event `StopMushroomAttack`
  ;[1 1 1] Handle mushroom attack
  (`KismetSystemLibrary.K2_InvalidateTimerHandle` (`self.MushroomAttackTimer`)))

(fn `UserConstructionScript`)